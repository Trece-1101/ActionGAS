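; GA_Primary is the player's primary melee attack gameplay ability.
; On activation it applies a block-hit-react effect, removed when the ability ends, and alternates two attack montages via FlipFlop, ending when the montage finishes or is interrupted.
; A Player.Primary gameplay event triggers a forward hitbox overlap test, which sends hit events to overlapped actors and applies ability-level damage effects to those with ability system components.
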(event `self.K2_ActivateAbility`
  (bind _returnvalue (`self.GetAbilitySystemComponentFromActorInfo`))
  (bind _returnvalue_2 (`self.GetAbilitySystemComponentFromActorInfo`))
  (`|ExecutionSequence`
    (:`then_0`
      ; Apply Block
      (`AbilitySystemComponent.BP_ApplyGameplayEffectSpecToSelf` _returnvalue_2 (`AbilitySystemComponent.MakeOutgoingSpec` :`self` _returnvalue_2 :`GameplayEffectClass` "/Game/CourseContent/AbilitySystem/GameplayEffects/Player/GE_BlockHitReact.GE_BlockHitReact_C" :`Level` 1.0)))
    (:`then_1`
      ;[0.00791 0.01273 0.15 0.5] Play Attack Montage
      (`/Engine/EditorBlueprintResources/StandardMacros.FlipFlop`
        (:`A`
          (`AbilityTask_PlayMontageAndWait.CreatePlayMontageAndWaitProxy` "None" (`self.AttackMontageA`)
            (:`OnCompleted`
              _)
            (:`OnBlendOut`
              _)
            (:`OnInterrupted`
              _)
            (:`OnCancelled`
              _)))
        (:`B`
          (`AbilityTask_PlayMontageAndWait.CreatePlayMontageAndWaitProxy` "None" (`self.AttackMontageB`)
            (:`OnCompleted`
              _)
            (:`OnBlendOut`
              _)
            (:`OnInterrupted`
              _)
            (:`OnCancelled`
              _))))
      (`self.K2_EndAbility`))
    (:`then_2`
      (`AbilityTask_WaitGameplayEvent.WaitGameplayEvent` (struct :`TagName` "CCTags.Events.Player.Primary") null
        (:`EventReceived`
          (bind _returnvalue_3 (`CC_BlueprintFunctionLib.HitBoxOverlapTest` (`self.GetAvatarActorFromActorInfo`) (`self.HitBoxForwardOffset`) (`self.HitBoxUpOffset`) (`self.HitBoxRadius`) (`self.bShowDebug`)))
          (`self.SendHitEventToActors` _returnvalue_3)
          (for _array_element _returnvalue_3
            (`/Engine/EditorBlueprintResources/StandardMacros.IsValid` _returnvalue
              (:`Is Valid`
                (bind _returnvalue_4 (`AbilitySystemBlueprintLibrary.GetAbilitySystemComponent` _array_element))
                (`/Engine/EditorBlueprintResources/StandardMacros.IsValid` _returnvalue_4
                  (:`Is Valid`
                    (`AbilitySystemComponent.BP_ApplyGameplayEffectSpecToTarget` _returnvalue (`AbilitySystemComponent.MakeOutgoingSpec` :`self` _returnvalue :`GameplayEffectClass` "/Game/CourseContent/AbilitySystem/GameplayEffects/Player/GE_PlayerDamage.GE_PlayerDamage_C" :`Level` (`KismetMathLibrary.Conv_IntToDouble` (`self.GetAbilityLevel`))) _returnvalue_4)))))))))))

(event `self.K2_OnEndAbility`
  (params (bWasCancelled :type Boolean))
  (`self.BP_RemoveGameplayEffectFromOwnerWithGrantedTags` (struct :`GameplayTags` (struct :`(TagName` "CCTags.CCAbilities.BlockHitReact"))) 1))
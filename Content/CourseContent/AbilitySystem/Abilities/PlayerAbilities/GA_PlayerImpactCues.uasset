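; Player gameplay ability that plays impact gameplay cues in response to hit and death events.
; On activation it waits in parallel for the player HitReact and Death gameplay events.
; HitReact executes the HitReact cue with the payload's effect context, instigator and source object.
; Death activates abilities tagged Death, then executes the BurstImpact cue on the avatar with the same payload data.
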(event `self.K2_ActivateAbility`
  (`|ExecutionSequence`
    (:`then_0`
      (bind (_asynctaskproxy _payload) (`AbilityTask_WaitGameplayEvent.WaitGameplayEvent` (struct :`TagName` "CCTags.CCEvents.Player.HitReact") null)
        (:`EventReceived`
          (`self.K2_ExecuteGameplayCueWithParams` (struct :`TagName` "GameplayCue.HitReact") (`AbilitySystemBlueprintLibrary.MakeGameplayCueParameters` 0.0 0.0 (`.ContextHandle` (break `GameplayEventData` _payload)) (struct) (struct) (struct) (struct) (0.0 0.0 0.0) (0.0 0.0 0.0) (`.Instigator` (break `GameplayEventData` _payload)) null (`.OptionalObject` (break `GameplayEventData` _payload)))))))
    (:`then_1`
      (bind (_asynctaskproxy_2 _payload_2) (`AbilityTask_WaitGameplayEvent.WaitGameplayEvent` (struct :`TagName` "CCTags.CCEvents.Player.Death") null)
        (:`EventReceived`
          (`AbilitySystemComponent.TryActivateAbilitiesByTag` (`self.GetAbilitySystemComponentFromActorInfo`) (`BlueprintGameplayTagLibrary.MakeGameplayTagContainerFromTag` (struct :`TagName` "CCTags.CCAbilities.Death")) true)
          (bind (_eventtag _instigator _target _optionalobject _optionalobject2 _contexthandle) (break `GameplayEventData` _payload_2))
          (`GameplayCueFunctionLibrary.ExecuteGameplayCueOnActor` (`self.GetAvatarActorFromActorInfo`) (struct :`TagName` "GameplayCue.BurstImpact") (`AbilitySystemBlueprintLibrary.MakeGameplayCueParameters` 0.0 0.0 _contexthandle (struct) (struct) (struct) (struct) (0.0 0.0 0.0) (0.0 0.0 0.0) _instigator null _optionalobject)))))))
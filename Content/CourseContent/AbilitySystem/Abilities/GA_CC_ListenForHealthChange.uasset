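; Gameplay ability that watches for health attribute changes and triggers death when the value runs out.
; On activation it starts a ListenForAttributeChange async task on the owner's Ability System Component, keeping a reference to end it when the ability ends.
; Each change can print old and new values for debugging; a new value at or below zero activates abilities by the Death tag.
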(event `self.K2_ActivateAbility`
  (bind _asc (`self.ASC`))
  (bind _output_get (set `self.ASC` (`self.GetAbilitySystemComponentFromActorInfo`)))
  (bind (_asynctaskproxy _attribute _newvalue _oldvalue) (`CC_AttributeChangeTask.ListenForAttributeChange` _output_get (struct :`AttributeName` "Health" :`Attribute` "/Script/GAS_Course.CC_AttributeSet:Health" :`AttributeOwner` "/Script/CoreUObject.Class'/Script/GAS_Course.CC_AttributeSet'"))
    (:`then`
      (set `self.AttributeChangedTask` _asynctaskproxy))
    (:`OnAttributeChanged`
      (`self.DebugHealth` _attribute _newvalue _oldvalue)
      (if (<= _newvalue 0.0)
        (`/Engine/EditorBlueprintResources/StandardMacros.IsValid` _asc
          (:`Is Valid`
            (`AbilitySystemComponent.TryActivateAbilitiesByTag` _asc (`BlueprintGameplayTagLibrary.MakeGameplayTagContainerFromTag` (struct :`TagName` "CCTags.CCAbilities.Death")) true)))))))

(event `self.K2_OnEndAbility`
  (params (bWasCancelled :type Boolean))
  (bind _attributechangedtask (`self.AttributeChangedTask`)
    (:`then`
      (`CC_AttributeChangeTask.EndTask` _attributechangedtask))
    (:`else`)))

(fn `DebugHealth`
  (params (GameplayAttribute :type "GameplayAttribute Structure (by ref)") (InDouble :type "Float (double-precision)") (InDouble2 :type "Float (double-precision)"))
  (`self.bShowDebug`
    (:`then`
      (`KismetSystemLibrary.PrintString` (`KismetStringLibrary.Concat_StrStr` "Old Value = " (`KismetStringLibrary.Conv_DoubleToString` InDouble2) "|| New Value = " (`KismetStringLibrary.Conv_DoubleToString` InDouble) "|| On Attribute" (`.AttributeName` (break `GameplayAttribute` GameplayAttribute))) true false (struct :`R` 1.0 :`G` 0.290326 :`A` 1.0) 3.0))
    (:`else`)))
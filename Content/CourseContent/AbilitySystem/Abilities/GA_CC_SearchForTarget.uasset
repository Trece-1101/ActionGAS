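; Gameplay Ability that drives an enemy's combat loop of finding, approaching and attacking a target.
; After a random per-enemy delay it finds the closest tagged actor in search range, retrying until one is alive.
; AIMoveTo closes in with a randomized acceptance radius, then the enemy rotates and activates its attack ability by tag.
; An EndAttack gameplay event restarts the search, and being launched blocks searching and attacking.
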(event `self.K2_ActivateAbility`
  (`|ExecutionSequence`
    (:`then_0`
      ; Cache Avatar and AI Controller
      (bind _ascc_enemy_character (cast `CC_EnemyCharacter` (`self.GetAvatarActorFromActorInfo`)))
      (bind _output_get (set `self.OwningEnemy` _ascc_enemy_character))
      (set `self.OwningAIController` (`AIBlueprintHelperLibrary.GetAIController` _output_get)))
    (:`then_1`
      (`self.StartSearch`))
    (:`then_2`
      ; Search After Attack
      (`AbilityTask_WaitGameplayEvent.WaitGameplayEvent` (struct :`TagName` "CCTags.Events.Enemy.EndAttack") null
        (:`EventReceived`
          (`self.StartSearch`))))))

(event `StartSearch`
  (bind _closestactor (`self.ClosestActor`))
  (bind _owningenemy (`self.OwningEnemy`))
  (`self.bShowDebug`
    (:`then`
      (`KismetSystemLibrary.PrintString` "Starting Search for Target"))
    (:`else`
      _))
  (bind _owningenemy_2 (`self.OwningEnemy`)
    (:`then`
      (`CC_EnemyCharacter.bIsBeingLaunched` _owningenemy_2
        (:`then`)
        (:`else`
          (bind (_outmindelay _outmaxdelay) (message `CC_AttackableInterface.GetAttackDelay` _owningenemy_2))
          (`AbilityTask_WaitDelay.WaitDelay` (`KismetMathLibrary.RandomFloatInRange` _outmindelay _outmaxdelay)
            (:`OnFinish`
              (`|ExecutionSequence`
                (:`then_0`
                  ; Find Target
                  (bind _returnvalue (`CC_BlueprintFunctionLib.FindClosestActorWithTag` _owningenemy (`Actor.K2_GetActorLocation` _owningenemy) (`self.Tag`) (`CC_BaseCharacter.SearchRange` _owningenemy)))
                  (set `self.ClosestActor` (break `ClosestActorWithTagResult` _returnvalue)))
                (:`then_1`
                  ; Attack
                  (`/Engine/EditorBlueprintResources/StandardMacros.IsValid` _closestactor
                    (:`Is Valid`
                      (`CC_BaseCharacter.bIsAlive` _closestactor
                        (:`then`
                          (`self.MoveToTargetAndAttack`))
                        (:`else`
                          (`self.StartSearch`))))
                    (:`Is Not Valid`
                      (`self.StartSearch`))))))))))
    (:`else`)))

(event `MoveToTargetAndAttack`
  (bind _arealive (`self.CheckActorAndOwner`))
  (if _arealive
    (bind _closestactor (`self.ClosestActor`)
      (:`then`
        (bind _owningaicontroller (`self.OwningAIController`)
          (:`then`
            (bind _owningenemy (`self.OwningEnemy`)
              (:`then`
                ; Attack When In position
                (bind _returnvalue (message `CC_AttackableInterface.GetAcceptanceRadius` _owningenemy))
                (`AITask_MoveTo.AIMoveTo` _owningaicontroller (0.0 0.0 0.0) _closestactor (+ _returnvalue (`KismetMathLibrary.RandomFloatInRange` 10.0 50.0))
                  (:`OnMoveFinished`
                    (`self.AttackTarget`))))
              (:`else`)))
          (:`else`)))
      (:`else`
        (`self.StartSearch`)))
    (else
      (`self.StartSearch`))))

(event `AttackTarget`
  (bind _closestactor (`self.ClosestActor`))
  (bind _asbp_enemy_base (cast `/Game/CourseContent/Characters/Enemies/BP_Enemy_Base` (`self.OwningEnemy`)))
  (`CC_EnemyCharacter.bIsBeingLaunched` _asbp_enemy_base
    (:`then`)
    (:`else`
      ; Rotate to target and Attack
      (`/Engine/EditorBlueprintResources/StandardMacros.IsValid` _closestactor
        (:`Is Valid`
          (`CC_EnemyCharacter.RotateToTarget` _asbp_enemy_base _closestactor)
          (`AbilityTask_WaitDelay.WaitDelay` (`TimelineComponent.GetTimelineLength` (`/Game/CourseContent/Characters/Enemies/BP_Enemy_Base.RotationTimeLine` _asbp_enemy_base))
            (:`OnFinish`
              (`AbilitySystemComponent.TryActivateAbilitiesByTag` (`AbilitySystemBlueprintLibrary.GetAbilitySystemComponent` (`self.OwningEnemy`)) (`BlueprintGameplayTagLibrary.MakeGameplayTagContainerFromTag` (struct :`TagName` "CCTags.CCAbilities.Enemy.Attack")) true))))))))

(fn `CheckActorAndOwner`
  (returns (AreAlive :type Boolean))
  (bind _owningenemy (`self.OwningEnemy`)
    (:`then`
      (return (and (`CC_BaseCharacter.bIsAlive` _owningenemy) (`CC_BaseCharacter.bIsAlive` (`self.ClosestActor`)))))
    (:`else`)))
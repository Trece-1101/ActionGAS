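; Gameplay ability that handles character death, then either respawns the character or retires it.
; It plays a death montage while applying GE_Death to itself, and branches on ShouldRespawn when the montage completes, is interrupted or is cancelled.
; Respawn removes Dead-tagged effects, sends an EndAttack event, resets attributes and moves to a player start on authority, then ends the ability.
; Non-respawning characters are hidden and given a lifespan.
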(event `self.K2_ActivateAbility`
  (bind _returnvalue (`self.GetAvatarActorFromActorInfo`))
  (bind _returnvalue_2 (`self.GetAbilitySystemComponentFromActorInfo`))
  (`AbilityTask_PlayMontageAndWait.CreatePlayMontageAndWaitProxy` "None" (`self.DeathMontage`)
    (:`then`
      (`AbilitySystemComponent.BP_ApplyGameplayEffectSpecToSelf` _returnvalue_2 (`AbilitySystemComponent.MakeOutgoingSpec` :`self` _returnvalue_2 :`GameplayEffectClass` "/Game/CourseContent/AbilitySystem/GameplayEffects/GE_Death.GE_Death_C" :`Level` 1.0)))
    (:`OnCompleted`
      (bind _ascc_base_character (cast `CC_BaseCharacter` _returnvalue :!label _label))
      (`CC_BaseCharacter.bShouldRespawn` _ascc_base_character
        (:`then`
          (`self.RespawnCharacter`))
        (:`else`
          (`Actor.SetLifeSpan` _returnvalue (`self.In Lifespan`))
          (`Actor.SetActorHiddenInGame` _returnvalue true))))
    (:`OnInterrupted`
      (goto _label))
    (:`OnCancelled`
      (goto _label))))

(event `RespawnCharacter`
  (`|ExecutionSequence`
    (:`then_0`
      (`self.BP_RemoveGameplayEffectFromOwnerWithGrantedTags` (struct :`GameplayTags` (struct :`(TagName` "CCTags.Status.Dead"))))
      (`AbilitySystemBlueprintLibrary.SendGameplayEventToActor` (`self.GetAvatarActorFromActorInfo`) (struct :`TagName` "CCTags.CCEvents.Enemy.EndAttack")))
    (:`then_1`
      ; Cache Base Character
      (bind _ascc_base_character (cast `CC_BaseCharacter` (`self.GetAvatarActorFromActorInfo`)))
      (set `self.BaseCharacter` _ascc_base_character))
    (:`then_2`
      (`self.K2_HasAuthority`
        (:`True`
          (`|ExecutionSequence`
            (:`then_0`
              ; Reset Attributes
              (bind _basecharacter (`self.BaseCharacter`)
                (:`then`
                  (`CC_BaseCharacter.ResetAttributes` _basecharacter))
                (:`else`)))
            (:`then_1`
              ; Respawn Character
              (bind _basecharacter_2 (`self.BaseCharacter`)
                (:`then`
                  (`Actor.K2_SetActorLocation` _basecharacter_2 (`Actor.K2_GetActorLocation` (`GameModeBase.K2_FindPlayerStart` (`GameplayStatics.GetGameMode`) (`Pawn.GetController` _basecharacter_2) "")) false false))
                (:`else`)))))))
    (:`then_3`
      (bind _basecharacter_3 (`self.BaseCharacter`)
        (:`then`
          (`CC_BaseCharacter.HandleRespawn` _basecharacter_3))
        (:`else`)))
    (:`then_4`
      (`self.K2_EndAbility`))))
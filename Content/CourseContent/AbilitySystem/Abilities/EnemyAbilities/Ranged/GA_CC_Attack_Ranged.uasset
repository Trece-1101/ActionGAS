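; Gameplay ability for an enemy ranged attack that plays an attack montage and fires a projectile.
; As the montage starts, it spawns BP_CC_Projectile at the Muzzle_Front socket, flattened to horizontal aim, passing in the avatar as owner and the Damage value.
; It immediately sends an EndAttack gameplay event to the avatar, while the ability itself ends when the montage completes, is interrupted or is cancelled.
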(event `self.K2_ActivateAbility`
  (bind _returnvalue (`self.GetAvatarActorFromActorInfo`))
  (bind (_returnvalue_location _returnvalue_rotation) (`KismetMathLibrary.BreakTransform` (`SceneComponent.GetSocketTransform` (`self.GetOwningComponentFromActorInfo`) "Muzzle_Front" "RTS_World")))
  (bind (_returnvalue_x _returnvalue_y) (`KismetMathLibrary.BreakVector` (`KismetMathLibrary.GetForwardVector` _returnvalue_rotation)))
  (`AbilityTask_PlayMontageAndWait.CreatePlayMontageAndWaitProxy` "None" "/Game/CourseContent/Characters/Enemies/Animations/Ranged/AM_Attack_Enemy_Ranged.AM_Attack_Enemy_Ranged" 1.0 "None" false
    (:`then`
      (`|SpawnActorFromClass` "/Game/CourseContent/GameObjects/Projectiles/BP_CC_Projectile.BP_CC_Projectile_C" (`KismetMathLibrary.MakeTransform` _returnvalue_location (`KismetMathLibrary.MakeRotFromX` (`KismetMathLibrary.MakeVector` _returnvalue_x _returnvalue_y))) "Undefined" "MultiplyWithRoot" _returnvalue (`self.Damage`) null)
      (`AbilitySystemBlueprintLibrary.SendGameplayEventToActor` _returnvalue (struct :`TagName` "CCTags.Events.Enemy.EndAttack")))
    (:`OnCompleted`
      (`self.K2_EndAbility` :!label _label))
    (:`OnInterrupted`
      (goto _label))
    (:`OnCancelled`
      (goto _label))))
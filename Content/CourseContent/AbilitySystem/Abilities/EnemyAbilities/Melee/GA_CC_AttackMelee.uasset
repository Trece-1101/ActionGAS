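; Enemy melee attack gameplay ability that ends immediately if the owner has the Dead tag.
; It plays a random montage from its list and ends when that montage completes, is interrupted or is cancelled.
; In parallel it waits once for a MeleeTraceHit event, then sends SetByCaller melee damage and impact particles to the hit player, with optional debug sphere.
; On ending, it sends an EndAttack event to its avatar.
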(event `self.K2_ActivateAbility`
  (if (not (`GameplayTagAssetInterface.HasMatchingGameplayTag` (`self.GetAbilitySystemComponentFromActorInfo`) (struct :`TagName` "CCTags.Status.Dead")))
    (`|ExecutionSequence`
      (:`then_0`
        (`AbilityTask_PlayMontageAndWait.CreatePlayMontageAndWaitProxy` "None" (`KismetArrayLibrary.Array_Random` (`self.Montages`)) 1.0 "None" false 1.0 0.0 true
          (:`OnCompleted`
            _)
          (:`OnInterrupted`
            _)
          (:`OnCancelled`
            _))
        (`self.K2_EndAbility`))
      (:`then_1`
        (bind (_asynctaskproxy _payload) (`AbilityTask_WaitGameplayEvent.WaitGameplayEvent` (struct :`TagName` "CCTags.CCEvents.Enemy.MeleeTraceHit") null true)
          (:`EventReceived`
            (`self.bShowDebug`
              (:`then`
                (bind (_eventtag _instigator _target _optionalobject _optionalobject2 _contexthandle) (break `GameplayEventData` _payload))
                (bind (_returnvalue_bblockinghit _returnvalue_binitialoverlap _returnvalue_time _returnvalue_distance _returnvalue_location _returnvalue_impactpoint) (`GameplayStatics.BreakHitResult` (`AbilitySystemBlueprintLibrary.EffectContextGetHitResult` _contexthandle)))
                (`KismetSystemLibrary.DrawDebugSphere` _returnvalue_impactpoint 40.0 12 (struct :`R` 0.089438 :`G` 0.848958 :`B` 0.156049 :`A` 1.0) 4.0 1.0))
              (:`else`
                _))
            (`CC_BlueprintFunctionLib.SendDamageEventToPlayer` _target (`self.Damage Effect`) _payload (`BlueprintGameplayTagLibrary.MakeLiteralGameplayTag` (struct :`TagName` "CCTags.SetByCaller.Melee")) (`self.Damage`) (`BlueprintGameplayTagLibrary.MakeLiteralGameplayTag` (struct :`TagName` "CCTags.None")) (`self.ImpactParticles`))))))
    (else
      (`self.K2_EndAbility`))))

(event `self.K2_OnEndAbility`
  (params (bWasCancelled :type Boolean))
  (`AbilitySystemBlueprintLibrary.SendGameplayEventToActor` (`self.GetAvatarActorFromActorInfo`) (struct :`TagName` "CCTags.Events.Enemy.EndAttack")))
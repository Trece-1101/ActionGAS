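; Enemy gameplay ability that plays a directional hit reaction montage when the enemy is hit.
; On activation it waits for the HitReact gameplay event and ignores it if the owner has the Dead tag.
; It compares avatar forward with the direction to the instigator, passes the result to the avatar, and jumps the montage to the matching named section.
; Optional debug prints show the event source and hit direction.
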(event `self.K2_ActivateAbility`
  (bind (_asynctaskproxy _payload) (`AbilityTask_WaitGameplayEvent.WaitGameplayEvent` (struct :`TagName` "CCTags.CCEvents.Enemy.HitReact") null)
    (:`EventReceived`
      (if (not (`GameplayTagAssetInterface.HasMatchingGameplayTag` (`self.GetAbilitySystemComponentFromActorInfo`) (struct :`TagName` "CCTags.Status.Dead")))
        (`self.DebugReceiveDamage` _payload)
        (`self.CacheHitDirectionVectors` (`.Instigator` (break `GameplayEventData` _payload)))
        (bind _outputpin (`self.CalculateHitDirection`))
        (`|ExecutionSequence`
          (:`then_0`
            ;[0.15 0.05859 0.05859 0.5] Debug
            (`self.bShowDebug`
              (:`then`
                (`KismetSystemLibrary.PrintString` (`KismetStringLibrary.Concat_StrStr` "Receiving Damage from: " (`KismetStringLibrary.Conv_NameToString` _outputpin)) true true (struct :`R` 1.0 :`B` 0.118841 :`A` 1.0)))
              (:`else`)))
          (:`then_1`
            ; Play Montage
            (`AbilityTask_PlayMontageAndWait.CreatePlayMontageAndWaitProxy` "None" (`self.HitReactMontage`)
              (:`then`
                (`self.MontageJumpToSection` (`self.HitDirectionName`))))))))))

(fn `CalculateHitDirection`
  (returns (OutputPin :type Name))
  (bind _returnvalue (`CC_BlueprintFunctionLib.GetHitDirection` (`self.AvatarForward`) (`self.ToInstigator`)))
  (bind _output_get (set `self.HitDirectionName` (`CC_BlueprintFunctionLib.GetHitDirectionName` _returnvalue)))
  (message `CC_DamageableInterface.SetLastHitDirection` (`self.GetAvatarActorFromActorInfo`) _returnvalue)
  (return _output_get))

(fn `DebugReceiveDamage`
  (params (GameplayEventData :type "GameplayEventData Structure (by ref)"))
  (bind (_eventtag _instigator _target) (break `GameplayEventData` GameplayEventData))
  (`self.bShowDebug`
    (:`then`
      (`KismetSystemLibrary.PrintString` (`KismetStringLibrary.Concat_StrStr` "GA_CC_HitReact: Received Event From: " (`KismetSystemLibrary.GetDisplayName` _instigator) "  Received In: " (`KismetSystemLibrary.GetDisplayName` _target)) true true (struct :`G` 0.013348 :`B` 1.0 :`A` 1.0) 3.0))
    (:`else`)))
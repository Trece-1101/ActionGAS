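; Base enemy Blueprint that handles item drops, last-hit tracking and turning to face a target.
; On destruction, it rolls against DropChance and spawns a random class from Drops at its own transform.
; RotatetoTarget plays a timeline that drives a quaternion slerp toward the target, with Z zeroed in the look-at to keep the enemy level.
; It stores the last hit direction through an event and exposes it through a getter.
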(event `self.ReceiveBeginPlay`
  (add `self.OnDestroyed` (delegate `EnemyDestroyed`)))

(event `EnemyDestroyed` :!signature `self.OnDestroyed`
  (params (DestroyedActor :type "Actor Object Reference"))
  (if (<= (`KismetMathLibrary.RandomFloatInRange` 0.0 1.0) (`self.DropChance`))
    (bind _result (`BlueprintSetLibrary.Set_ToArray` (`self.Drops`)))
    (`|SpawnActorFromClass` (`KismetArrayLibrary.Array_Random` _result) (`self.GetTransform`) "AdjustIfPossibleButAlwaysSpawn" "MultiplyWithRoot" null null)))

(event `CC_DamageableInterface.SetLastHitDirection`
  (params (HitDirection :type "EHitDirection Enum" :default "Front"))
  (set `self.Hit Direction` HitDirection))

(event `self.RotateToTarget`
  (params (Target :type "Actor Object Reference"))
  (bind (_direction _rotatetrack) (`Timeline|RotationTimeLine` :!via `PlayFromStart`)
    (:`Update`
      (`self.SetFacingRotation` Target _rotatetrack))))

(fn `GetLastHitDirection`
  (returns (ReturnValue :type "EHitDirection Enum"))
  (return (`self.Hit Direction`)))

(fn `SetFacingRotation`
  (params (RotateTarget :type "Actor Object Reference") (Alpha :type "Float (double-precision)"))
  (bind (_returnvalue_x _returnvalue_y) (`KismetMathLibrary.BreakVector` (`self.K2_GetActorLocation`)))
  (bind (_returnvalue_x_2 _returnvalue_y_2) (`KismetMathLibrary.BreakVector` (`self.K2_GetActorLocation` (`local.RotateTarget`))))
  (`local.RotateTarget`
    (:`then`
      (`self.K2_SetActorRotation` (`KismetMathLibrary.Quat_Rotator` (`KismetMathLibrary.Quat_Slerp` (`KismetMathLibrary.Conv_RotatorToQuaternion` (`self.K2_GetActorRotation`)) (`KismetMathLibrary.Conv_RotatorToQuaternion` (`KismetMathLibrary.FindLookAtRotation` (`KismetMathLibrary.MakeVector` _returnvalue_x _returnvalue_y) (`KismetMathLibrary.MakeVector` _returnvalue_x_2 _returnvalue_y_2))) (`local.Alpha`)))))
    (:`else`)))

(fn `UserConstructionScript`)
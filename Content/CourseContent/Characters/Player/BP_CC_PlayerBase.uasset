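; Base player character Blueprint that connects the Gameplay Ability System to the player's HUD.
; BeginPlay binds to the ASC-initialized event and also runs the handler immediately if the component is already valid, covering either initialization order.
; The handler casts the ASC, attribute set, controller and HUD, then passes the first two to BP_HUD's SetupPlayerUI.
; The L key acts as a debug input that levels up GA_Primary and prints the new level.
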(event `self.ReceiveBeginPlay`
  (bind _returnvalue (`AbilitySystemBlueprintLibrary.GetAbilitySystemComponent` null))
  (add `self.OnAbilitySystemComponentInitialized` (delegate `OnGASReady`))
  (`/Engine/EditorBlueprintResources/StandardMacros.IsValid` _returnvalue
    (:`Is Valid`
      (`self.OnGASReady` _returnvalue (`self.GetAttributeSet`)))))

(event `OnGASReady` :!signature `self.OnAbilitySystemComponentInitialized`
  (params (AbilitySystemComponent :type "AbilitySystemComponent Object Reference") (AttributeSet :type "AttributeSet Object Reference"))
  (bind _ascc_ability_system_component (cast `CC_AbilitySystemComponent` AbilitySystemComponent))
  (bind _ascc_attribute_set (cast `CC_AttributeSet` AttributeSet))
  (bind _ascc_player_controler (cast `CC_PlayerControler` (`self.GetController`)))
  (bind _asbp_hud (cast `/Game/CourseContent/UI/BP_HUD` (`PlayerController.GetHUD` _ascc_player_controler)))
  (`/Game/CourseContent/UI/BP_HUD.SetupPlayerUI` _asbp_hud _ascc_ability_system_component _ascc_attribute_set))

(event `Key|L`
  (params (Key :type "Key Structure"))
  (:`Pressed`
    (bind _ascc_ability_system_component (cast `CC_AbilitySystemComponent` (`AbilitySystemBlueprintLibrary.GetAbilitySystemComponent` null)))
    (`CC_AbilitySystemComponent.AddToAbilityLevel` _ascc_ability_system_component "/Game/CourseContent/AbilitySystem/Abilities/PlayerAbilities/GA_Primary.GA_Primary_C" 1)
    (`KismetSystemLibrary.PrintString` (`KismetStringLibrary.Concat_StrStr` "New Level = " (`KismetStringLibrary.Conv_IntToString` (`CC_AbilitySystemComponent.GetAbilityLevelByClass` _ascc_ability_system_component "/Game/CourseContent/AbilitySystem/Abilities/PlayerAbilities/GA_Primary.GA_Primary_C"))))))

(fn `UserConstructionScript`)